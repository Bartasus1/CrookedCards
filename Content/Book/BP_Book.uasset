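; BP_Book is an in-world book actor whose pages display UMG widgets and can be turned with the keyboard.
; On BeginPlay it creates WB_Book, renders that widget's BookWidgetSwitcher onto the pages, takes input from player controller 0, then opens the first page after a short delay.
; Right and Left arrow keys call the page-turning functions, which are not defined in this graph.
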(event `self.ReceiveBeginPlay`
  (`parent.ReceiveBeginPlay`)
  (bind _returnvalue (`|CreateWidget` "/Game/UI/Book/WB_Book.WB_Book_C"))
  (`self.RenderWidgetToPages` (`/Game/UI/Book/WB_Book.BookWidgetSwitcher` _returnvalue))
  (`self.SetOwner` (`GameplayStatics.GetPlayerController` 0))
  (`self.EnableInput` (`GameplayStatics.GetPlayerController` 0))
  (`KismetSystemLibrary.Delay` 0.2)
  (`self.OpenPage` 0))

(event `Key|Right`
  (params (Key :type "Key Structure"))
  (:`Pressed`
    (`self.TurnNextPage`)))

(event `Key|Left`
  (params (Key :type "Key Structure"))
  (:`Pressed`
    (`self.TurnPrevPage`)))

(fn `UserConstructionScript`)