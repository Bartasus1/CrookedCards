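; BP_GameBoard is the game board Blueprint that places and initializes player bases and playable characters.
; It returns one of two fraction spawn point transforms, selected by player ID.
; Base initialization calls the parent logic, then applies an init Gameplay Effect through the base's Ability System Component.
; Playable character initialization applies its own init effect the same way, with no parent call.
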(fn `GetTransformForFraction`
  (params (PlayerID :type Integer))
  (returns (ReturnValue :type "Transform Structure"))
  (return (`SceneComponent.K2_GetComponentToWorld` (select `int` PlayerID :`0` (`self.FractionSpawnPoint0`) :`1` (`self.FractionSpawnPoint1`) :!type "SceneComponent Object Reference"))))

(fn `InitPlayableCharacter`
  (params (Character :type "KKCharacter Object Reference"))
  (`AbilitySystemComponent.BP_ApplyGameplayEffectToSelf` :`self` (`AbilitySystemBlueprintLibrary.GetAbilitySystemComponent` Character) :`GameplayEffectClass` "/Game/GameplayEffects/GE_InitPlayableCharacter.GE_InitPlayableCharacter_C"))

(fn `InitPlayerBase`
  (params (PlayerID :type Integer) (BaseCharacter :type "KKCharacter Object Reference"))
  (`parent.InitPlayerBase` PlayerID BaseCharacter)
  (`AbilitySystemComponent.BP_ApplyGameplayEffectToSelf` :`self` (`AbilitySystemBlueprintLibrary.GetAbilitySystemComponent` BaseCharacter) :`GameplayEffectClass` "/Game/GameplayEffects/GE_InitPlayerBase.GE_InitPlayerBase_C"))

(fn `UserConstructionScript`)