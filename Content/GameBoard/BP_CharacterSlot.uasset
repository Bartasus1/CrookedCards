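; BP_CharacterSlot is a game board slot that moves a character onto its own location.
; MoveCharacter defers to the parent implementation when ExecuteImmediateMovement is set.
; Otherwise a timeline interpolates the character from its start location to the slot with unswept teleports, then sends it a FinishedAction gameplay event through the Gameplay Ability System.
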(event `self.MoveCharacter`
  (params (Character :type "KKCharacter Object Reference"))
  (if (not (`self.bExecuteImmediateMovement`))
    (set `self.StartLocation` (`self.K2_GetActorLocation` Character))
    (bind (_direction _move) (`Timeline|MovementTimeLine` :!via `PlayFromStart`)
      (:`Update`
        (`self.K2_SetActorLocation` Character (`KismetMathLibrary.VLerp` (`self.StartLocation`) (`self.K2_GetActorLocation`) _move) false true))
      (:`Finished`
        (`AbilitySystemBlueprintLibrary.SendGameplayEventToActor` Character (struct :`TagName` "GameplayAbilitySystem.Events.FinishedAction"))))
    (else
      (`parent.MoveCharacter` Character))))

(fn `UserConstructionScript`)