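; BP_Pikinier is the pikeman character of the Zakon faction in a slot-based board game, with its own attack damage rule.
; Its only logic is the attacker damage calculation, which for the default attack type reads the game board distance between its slot and the target's.
; That distance indexes a Select: adjacent targets take the unit's Strength, while targets two slots away take a hard-coded amount independent of Strength.
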(fn `Attacker_CalculateDamage`
  (params (TargetCharacter :type "KKCharacter Object Reference") (AttackInfo :type "AttackInfo Object Reference"))
  (`|SwitchGameplayTag` (`AttackInfo.AttackType` AttackInfo)
    (:`AttackType.DefaultAttack`
      (bind _returnvalue (`KKGameBoard.GetDistanceBetweenSlots` (`self.GetGameBoard`) (`self.CharacterSlotID`) (`KKCharacter.CharacterSlotID` (`local.TargetCharacter`))))
      (set `AttackInfo.Damage` (select `byte` (`KismetMathLibrary.Conv_IntToByte` _returnvalue) :`0` 0.0 :`1` (`KismetMathLibrary.Conv_IntToDouble` (`self.GetStrength`)) :`2` 6.0 :!type "Float (single-precision)") (`local.AttackInfo`)))))

(fn `UserConstructionScript`)