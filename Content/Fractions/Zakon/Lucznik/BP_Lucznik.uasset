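; BP_Lucznik is the archer unit of the Zakon faction, whose attacks wear down enemy defence.
; The StrzałyRozrywające (tearing arrows) attack-stage event increments AttackCounter, and every second count resets it and lowers the victim's defence by one.
; AttackerOnAttackEnd repeats the same logic on its target character, sharing that counter.
; The counter is not tracked per target, so the penalty hits whoever receives the second count.
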(event `self.Strzały Rozrywające.AttackStageExecution`
  (params (AttackSequence :type "AttackSequence Object Reference"))
  (bind _output_get (set `self.AttackCounter` (+ (`self.AttackCounter`) 1)))
  (if (>= _output_get 2)
    (set `self.AttackCounter` 0)
    (`self.ModifyDefence` (`AttackSequence.GetVictim` AttackSequence) "Additive" -1.0)))

(fn `Attacker_OnAttackEnd`
  (params (TargetCharacter :type "KKCharacter Object Reference") (AttackInfo :type "AttackInfo Object Reference"))
  (bind _output_get (set `self.AttackCounter` (+ (`self.AttackCounter`) 1)))
  (if (>= _output_get 2)
    (set `self.AttackCounter` 0)
    (`self.ModifyDefence` (`local.TargetCharacter`) "Additive" -1.0)))

(fn `UserConstructionScript`)