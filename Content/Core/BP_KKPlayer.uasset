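; BP_KKPlayer is the player Blueprint with a cursor-directed camera zoom on its SpringArm.
; BeginPlay adds the default Enhanced Input mapping context when locally controlled.
; Starting IA_Zoom lowers the arm's target offset and shifts it toward the world point under the cursor, relative to the actor.
; While triggered, input pans that offset horizontally; completion resets it to zero.
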(event `self.ReceiveBeginPlay`
  (if (`self.IsLocallyControlled`)
    (`EnhancedInputSubsystemInterface.AddMappingContext` (pcsubsystem `EnhancedInputLocalPlayerSubsystem` (`GameplayStatics.GetPlayerController` 0)) "/Game/Core/Input/IMC_Default.IMC_Default" 0 (struct))))

(event `EnhancedInput|/Game/Core/Input/IA_Zoom`
  (params (ActionValue :type "Vector Structure") (ElapsedSeconds :type "Float (double-precision)") (TriggeredSeconds :type "Float (double-precision)") (InputAction :type "InputAction Object Reference" :default "/Game/Core/Input/IA_Zoom.IA_Zoom"))
  (bind (_targetoffset_x _targetoffset_y) (`KismetMathLibrary.BreakVector` (`SpringArmComponent.TargetOffset` (`self.SpringArm`))))
  (bind (_returnvalue_x _returnvalue_y) (`KismetMathLibrary.BreakVector` (- (`.Location` (`GameplayStatics.BreakHitResult` (`PlayerController.GetHitResultUnderCursorByChannel` (`GameplayStatics.GetPlayerController` 0) "TraceTypeQuery1" false))) (`self.K2_GetActorLocation`))))
  (:`Triggered`
    (set `SpringArmComponent.TargetOffset` (`KismetMathLibrary.MakeVector` (+ _targetoffset_x (.x ActionValue)) (+ _targetoffset_y (.y ActionValue)) -350.0) (`self.SpringArm`)))
  (:`Started`
    (set `SpringArmComponent.TargetOffset` (`KismetMathLibrary.MakeVector` _returnvalue_x _returnvalue_y -350.0) (`self.SpringArm`)))
  (:`Completed`
    (set `SpringArmComponent.TargetOffset` (0.0 0.0 0.0) (`self.SpringArm`))))

(fn `UserConstructionScript`)